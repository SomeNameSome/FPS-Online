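; Character Blueprint that holds debug test logic for weapon attachment and a mode-change montage, bound to the 5 key.
; Pressing 5 is wired both to print the current weapon's attach socket name through the Mylt event and to play ChangeMode_Montage on the mesh, printing on notify begin and end.
; Unconnected nodes for finding AK47 actors and snapping a weapon to the right-hand socket remain, and PrintWeaponListDebug is empty.
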(event `Key|Five`
  (params (Key :type "Key Structure"))
  (:`Pressed`
    (`self.mylt` (`self.CurrentWeapon`))))

(event `mylt`
  (params (NewParam :type "Weapon_Base Object Reference"))
  (`KismetSystemLibrary.PrintString` (`KismetStringLibrary.Conv_NameToString` (`self.GetAttachParentSocketName` NewParam)) true true (struct :`G` 0.66 :`B` 1.0 :`A` 1.0) 5.0))

(event `Key|Five`
  (params (Key :type "Key Structure"))
  (:`Pressed`
    (`|PlayMontage` (`self.Mesh`) "/Game/Person/Animations/ChangeMode/ChangeMode_Montage.ChangeMode_Montage"
      (:`OnNotifyBegin`
        (`KismetSystemLibrary.PrintString` "Begin"))
      (:`OnNotifyEnd`
        (`KismetSystemLibrary.PrintString` "End")))))

(fn `PrintWeaponListDebug`)

(fn `UserConstructionScript`)