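; StaticActorPrimaryBP is an actor Blueprint that gives impact feedback when it takes damage.
; Its damage event calls the GameState_Base spawn RPCs to place a decal oriented to the hit normal and a particle emitter at the hit location.
; GetParticleEffect picks a small, medium or large stone impact from the absolute damage, with no effect defined above the top range.
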(event `self.ITakeDamageBlueprint`
  (params (damage :type "Float (single-precision)") (InLocation :type "Vector Structure") (InNormal :type "Vector Structure"))
  (bind _asgame_state_base (cast `GameState_Base` (`GameplayStatics.GetGameState`)))
  (`GameState_Base.SpawnDecalRPC` _asgame_state_base "/Game/Weapon/DecalMaterial.DecalMaterial" InLocation (`KismetMathLibrary.MakeRotFromX` InNormal))
  (`GameState_Base.SpawnEmitterRPC` _asgame_state_base (`self.GetParticleEffect` damage) InLocation))

(fn `GetParticleEffect`
  (params (Damage :type "Float (double-precision)"))
  (returns (ParticleEffect :type "ParticleSystem Object Reference"))
  (bind _returnvalue (`KismetMathLibrary.Abs` Damage))
  (if (`KismetMathLibrary.InRange_FloatFloat` _returnvalue 0.0 15.0)
    (return "/Game/MilitaryWeapDark/FX/P_Impact_Stone_Small_01.P_Impact_Stone_Small_01")
    (elif (`KismetMathLibrary.InRange_FloatFloat` _returnvalue 15.0 50.0)
      (return "/Game/MilitaryWeapDark/FX/P_Impact_Stone_Medium_01.P_Impact_Stone_Medium_01")
      (elif (`KismetMathLibrary.InRange_FloatFloat` _returnvalue 50.0 100.0)
        (return "/Game/MilitaryWeapDark/FX/P_Impact_Stone_Large_01.P_Impact_Stone_Large_01")))))

(fn `UserConstructionScript`)